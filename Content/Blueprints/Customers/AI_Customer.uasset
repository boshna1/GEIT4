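; AI_Customer is a customer pawn Blueprint that picks up what is held on the board and leaves.
; On the Notify event it prints a ready message, finds the BP_Board actor and walks to its Target's location with AIMoveTo.
; After arriving and a short delay, it destroys the board's held object and walks back to its Spawn point.
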(event `/Game/Blueprints/Customers/BPI_Observer.Notify`
  (`KismetSystemLibrary.PrintString` "Ready!")
  (bind _returnvalue (`GameplayStatics.GetActorOfClass` "/Game/Blueprints/BP_Board.BP_Board_C"))
  (`|AIMoveTo` self (`self.K2_GetActorLocation` (`self.Target`)) null
    (:`then`
      (`KismetSystemLibrary.Delay` 0.8)
      (`self.K2_DestroyActor` (`/Game/Blueprints/BP_Board.HoldObj` _returnvalue))
      (`|AIMoveTo` self (`self.Spawn`) null))))

(fn `UserConstructionScript`)