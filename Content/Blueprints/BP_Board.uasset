(event `self.ReceiveBeginPlay`
  (`PhysicsHandleComponent.SetTargetLocation` (`self.PhysicsHandle`) (`SceneComponent.K2_GetComponentLocation` (`self.Sphere`))))

(event `self.ReceiveTick`
  (params (DeltaSeconds :type "Float (single-precision)")))

(fn `GetHeldObj`
  (params (Component :type "PrimitiveComponent Object Reference") (Item :type "/Game/Blueprints/Food/BP_BaseItem Object Reference"))
  (bind _returnvalue (`GameplayStatics.GetActorOfClass` "/Game/Blueprints/Player/BP_PlayerCharacter.BP_PlayerCharacter_C"))
  (`PhysicsHandleComponent.GrabComponentAtLocation` (`self.PhysicsHandle`) Component "None" (`/Game/Blueprints/Player/BP_PlayerCharacter.Hand` _returnvalue))
  (set `self.HoldObj` Item))

(fn `Make`
  (params (Item :type "/Game/Blueprints/Food/BP_BaseItem Object Reference"))
  (bind _holdobj (`self.HoldObj`))
  (bind _returnvalue (`SceneComponent.K2_GetComponentToWorld` (`self.Sphere`)))
  (`|ExecutionSequence`
    (:`then_0`
      (cast `/Game/Blueprints/Food/Ingredients/BP_BurgerBun` _holdobj)
      (cast `/Game/Blueprints/Food/Ingredients/BP_Pickle` Item)
      (bind _returnvalue_2 (`|SpawnActorFromClass` "/Game/Blueprints/Food/Dish/BP_PickleBurger.BP_PickleBurger_C" _returnvalue "Undefined" "MultiplyWithRoot" null null :!label _label))
      (set `self.HoldObj` _returnvalue_2))
    (:`then_1`
      (cast `/Game/Blueprints/Food/Ingredients/BP_Dog` _holdobj)
      (cast `/Game/Blueprints/Food/Ingredients/BP_HotdogBun` Item)
      (bind _returnvalue_3 (`|SpawnActorFromClass` "/Game/Blueprints/Food/Dish/BP_Hotdog.BP_Hotdog_C" _returnvalue "Undefined" "MultiplyWithRoot" null null :!label _label_2))
      (set `self.HoldObj` _returnvalue_3))
    (:`then_2`
      (cast `/Game/Blueprints/Food/Ingredients/BP_Pickle` _holdobj)
      (cast `/Game/Blueprints/Food/Ingredients/BP_BurgerBun` Item)
      (goto _label))
    (:`then_3`
      (cast `/Game/Blueprints/Food/Ingredients/BP_HotdogBun` _holdobj)
      (cast `/Game/Blueprints/Food/Ingredients/BP_Dog` Item)
      (goto _label_2)))
  (bind _outactors (`GameplayStatics.GetAllActorsOfClass` "/Game/Blueprints/Customers/AI_Customer.AI_Customer_C"))
  (for _array_element _outactors
    (`/Game/Blueprints/Customers/AI_Customer.Notify` _array_element)))

(fn `ObtainObj`)

(fn `UserConstructionScript`)